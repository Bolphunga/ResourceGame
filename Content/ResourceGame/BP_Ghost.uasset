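; BP_Ghost is a ghost character that replays a recorded path of timestamped locations and rotations.
; SetGhostPath0 stores the path, resets playback and snaps the ghost to the first frame.
; UpdateGhostPosition0 relies on an outside caller, advancing playback time by DeltaTime and lerping between neighboring frames until the last.
; Velocity experiments for animation are disconnected, and GetGhostSpeed returns a GhostSpeed variable that nothing here sets.
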(event `self.ReceiveTick`
  (params (DeltaSeconds :type "Float (single-precision)")))

(fn `GetGhostSpeed`
  (returns (Speed :type "Float (double-precision)"))
  (return (`self.GhostSpeed`)))

(fn `SetGhostPath0`
  (params (InPath :type "Array of GhostFrame Structure"))
  (bind _output_get (set `self.GhostPath0` InPath))
  (set `self.GhostPlaybackTime0` 0.0)
  (set `self.CurrentFrameIndex0` 0)
  (if (`KismetArrayLibrary.Array_IsNotEmpty` _output_get)
    (bind (_timestamp _location _rotation) (break `GhostFrame` (`|GetArrayItem` _output_get)))
    (`self.K2_SetActorLocationAndRotation` _location _rotation)
    (return)))

(fn `UpdateGhostPosition0`
  (params (DeltaTime :type "Float (double-precision)"))
  (locals (FrameDelta :type "Float (double-precision)"))
  (bind _ghostpath0 (`self.GhostPath0`))
  (bind _currentframeindex0 (`self.CurrentFrameIndex0`))
  (bind _returnvalue (`KismetArrayLibrary.Array_Length` (`self.GhostPath0`)))
  (bind (_timestamp _location _rotation) (break `GhostFrame` (`|GetArrayItem` _ghostpath0 _currentframeindex0)))
  (bind (_timestamp_2 _location_2 _rotation_2) (break `GhostFrame` (`|GetArrayItem` _ghostpath0 (+ _currentframeindex0 1))))
  (bind _returnvalue_2 (- _timestamp_2 _timestamp))
  ; If the GhostPath array is less than two frames or the index is >= 1, return.
  (if (or (< _returnvalue 2) (>= (`self.CurrentFrameIndex0`) (- _returnvalue 1)))
    (return)
    (else
      (bind _output_get (set `self.GhostPlaybackTime0` (+ DeltaTime (`self.GhostPlaybackTime0`))))
      (if (<= _returnvalue_2 0.0)
        (set `local.FrameDelta` 0.01))
      (bind _returnvalue_3 (/ (- _output_get _timestamp) _returnvalue_2))
      (`self.K2_SetActorLocation` (`KismetMathLibrary.VLerp` _location _location_2 _returnvalue_3))
      (`self.K2_SetActorRotation` (`KismetMathLibrary.RLerp` _rotation _rotation_2 _returnvalue_3))
      (if (>= (`self.GhostPlaybackTime0`) _timestamp_2)
        (set `self.CurrentFrameIndex0` (+ (`self.CurrentFrameIndex0`) 1))))))

(fn `UserConstructionScript`)