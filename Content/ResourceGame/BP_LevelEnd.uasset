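; BP_LevelEnd is a level-finish trigger that ends the current run when the player reaches it.
; Its CollisionBox overlap checks that the overlapping actor is player 0's BP_ThirdPersonCharacter, then calls EndCurrentRun on BP_ThirdPersonGameMode.
; It then prints the current level name and the next level name from BP_GhostGameInstance as debug output, without loading a level itself.
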(event `self.CollisionBox.OnComponentBeginOverlap`
  (params (OverlappedComponent :type "PrimitiveComponent Object Reference") (OtherActor :type "Actor Object Reference") (OtherComp :type "PrimitiveComponent Object Reference") (OtherBodyIndex :type Integer) (bFromSweep :type Boolean) (SweepResult :type "HitResult Structure (by ref)"))
  (bind _asbp_third_person_character (cast `/Game/ThirdPerson/Blueprints/BP_ThirdPersonCharacter` (`GameplayStatics.GetPlayerPawn` 0)))
  (bind _asbp_third_person_game_mode (cast `/Game/ThirdPerson/Blueprints/BP_ThirdPersonGameMode` (`GameplayStatics.GetGameMode`)))
  (if (== _asbp_third_person_character OtherActor)
    (`AGameModeBase.EndCurrentRun` _asbp_third_person_game_mode)
    (bind _asbp_ghost_game_instance (cast `/Game/ResourceGame/BP_GhostGameInstance` (`GameplayStatics.GetGameInstance`)))
    (bind _returnvalue (`GameplayStatics.GetCurrentLevelName` true))
    (`KismetSystemLibrary.PrintString` _returnvalue)
    (`KismetSystemLibrary.PrintString` (`KismetStringLibrary.Conv_NameToString` (`SGhostGameInstance.GetNextLevelName` _asbp_ghost_game_instance)))))

(fn `UserConstructionScript`)